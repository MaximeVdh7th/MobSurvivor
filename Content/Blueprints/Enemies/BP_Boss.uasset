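; Boss enemy Blueprint that deals contact damage, reacts to weapon projectile hits, spawns damage zones and toggles a spin pose.
; Collision overlap calls Damage on the other actor, then TakeDamages for weapon projectiles.
; The spin toggle flip-flops two cubes' pose while timelines ramp SpinRadius up or down and ease the pivot's yaw back afterwards.
; BeginPlay forces a fixed spawn height as a temporary bug fix.
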(event OnComponentBeginOverlap(Collision)
  (params (OverlappedComponent :type Primitive%20Component%20Object%20Reference) (OtherActor :type Actor%20Object%20Reference) (OtherComp :type Primitive%20Component%20Object%20Reference) (OtherBodyIndex :type Integer) (bFromSweep :type Boolean) (SweepResult :type Hit%20Result%20Structure%20%28by%20ref%29))
  ;[1 1 1] Call Trigger event damage
  (Utilities|FlowControl|Sequence
    (:then_0
      (Class|Boss|Damage OtherActor))
    (:then_1
      (bind _asweapon_projectile_bp (Utilities|Casting|CastToWeaponProjectile_BP OtherActor))
      (Class|Boss|TakeDamages _asweapon_projectile_bp))))

(event EventBeginPlay
  (bind _returnvalue (Transformation|GetActorLocation))
  ;[1 1 1 0.307] temporary fix of Height spawn bug
  (Transformation|SetActorLocation (Math|Vector|MakeVector (.x _returnvalue) (.y _returnvalue) 1.3e+02) false false))

(event EventSpinColliderToggle
  (bind _cube2 (Variables|Default|GetCube2))
  (bind _cube2_2 (Variables|Default|GetCube2))
  ;[0.5149 1 0 0.246] Spin mechanic
  ;;[1 1 1] Flip flop T-Pose blocking
  (Utilities|FlowControl|FlipFlop
    (:A
      (Transformation|AddLocalOffset _cube2_2 "0.000000,0.000000,32.000000" false false)
      (Transformation|SetRelativeRotation _cube2_2 "90.000000,0.000000,0.000000" false false)
      ;;[1 1 1] Smooth interpolation of spinning
      (bind _multiplier (Timeline|Radius Play)
        (:Update
          (Variables|Default|SetSpinRadius (* 5e+01 _multiplier)))))
    (:B
      (Transformation|SetRelativeRotation _cube2 "0, 0, 0" false false)
      (Transformation|AddLocalOffset _cube2 "0.000000,0.000000,-32.000000" false false)
      (Utilities|FlowControl|Sequence
        (:then_0
          (Timeline|Radius Reverse))
        (:then_1
          ;;[0.566 0.07239 1] Rotation Reset after Spin
          (bind _multiplier_2 (Timeline|RotationReset PlayFromStart)
            (:Update
              (Transformation|SetRelativeRotation (Variables|Default|GetPivotPoint) (Math|Rotator|MakeRotator 0.0 0.0 (Math|Float|Lerp (.yaw (Variables|/Script/Engine.SceneComponent|GetRelativeRotation (Variables|Default|GetPivotPoint))) -9e+01 _multiplier_2)) false false))))))))

(event EventSpawnDamageZone
  (params (Location :type Vector :default "0, 0, 0"))
  ;[1 1 1] Spawn Damage Zone BP
  (Game|SpawnActorfromClass "/Game/Blueprints/Enemies/BossDamageZone_BP.BossDamageZone_BP_C" (Math|Transform|MakeTransform (Math|Vector|MakeVector (.x Location) (.y Location) 1.1e+02) "0, 0, 0" "1.000000,1.000000,1.000000") "Undefined" "MultiplyWithRoot" 0 0))

(fn ConstructionScript)