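; BossDamageZone_BP is a timed damage zone actor for bosses that grows in, lingers, then shrinks away.
; On BeginPlay the Scale timeline plays forward while a ZoneDuration delay runs, then reverses and the actor destroys itself shortly after.
; Each timeline update scales the actor uniformly by ZoneRadius.
; No damage logic is in the graph; empty Collision overlap events are kept, per a comment, for C++ function calls.
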(event OnComponentBeginOverlap(Collision)
  (params (OverlappedComponent :type Primitive%20Component%20Object%20Reference) (OtherActor :type Actor%20Object%20Reference) (OtherComp :type Primitive%20Component%20Object%20Reference) (OtherBodyIndex :type Integer) (bFromSweep :type Boolean) (SweepResult :type Hit%20Result%20Structure%20%28by%20ref%29))
  ;[1 0.07812 0.07812 0.277] That MTF can't call c++ function without these Events (is he stupid ?)
)

(event OnComponentEndOverlap(Collision)
  (params (OverlappedComponent :type Primitive%20Component%20Object%20Reference) (OtherActor :type Actor%20Object%20Reference) (OtherComp :type Primitive%20Component%20Object%20Reference) (OtherBodyIndex :type Integer))
  ;[1 0.07812 0.07812 0.277] That MTF can't call c++ function without these Events (is he stupid ?)
)

(event EventBeginPlay
  (Utilities|FlowControl|Sequence
    (:then_0
      (Utilities|FlowControl|Delay (Variables|Default|GetZoneDuration))
      (Utilities|FlowControl|Sequence
        (:then_0
          (Utilities|FlowControl|Delay 0.5)
          (Actor|DestroyActor))
        (:then_1
          (bind _scale (Timeline|Scale ReverseFromEnd)
            (:Update
              (Transformation|SetActorScale3D (Math|Vector|MakeVector (* _scale (Variables|Default|GetZoneRadius)) (* _scale (Variables|Default|GetZoneRadius)) (* _scale (Variables|Default|GetZoneRadius)))))))))
    (:then_1
      (Timeline|Scale PlayFromStart))))

(fn ConstructionScript)