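; Player character Blueprint that owns the HUD, level-up screen, pause menu, abilities and death handling.
; It feeds Health and Experience components into the HUD; leveling up pauses the game and offers new bonuses.
; Cooldown-gated keys trigger a velocity-override dash with brief invincibility and an exploding bomb, using Delays.
; Debug keys adjust time dilation and toggle god mode, which blocks the one-time game-over call on death.
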(event Custom|OnLevelUp
  (params (NewLevel :type Integer))
  (Game|SetGamePaused true)
  (UserInterface|Viewport|AddtoViewport (Variables|Default|GetLevelUpUI) 0)
  (Default|GetANewSetOfBonuses (Variables|Default|GetLevelUpUI)))

(event Input|EnhancedActionEvents|EnhancedInputActionIA_Pause
  (params (ActionValue :type Boolean) (ElapsedSeconds :type Float%20%28double-precision%29) (TriggeredSeconds :type Float%20%28double-precision%29) (InputAction :type Input%20Action%20Object%20Reference :default "/Game/Input/Actions/IA_Pause.IA_Pause"))
  ;[0 1 0.09341] Pause Menu with P
  (:Started
    (if (not (Variables|Default|GetIsPauseMenuOpened))
      (Variables|Default|SetIsPauseMenuOpened true)
      (bind _returnvalue (UserInterface|CreateWidget "/Game/UI/PauseMenu_UW.PauseMenu_UW_C" (Game|GetPlayerController 0)))
      (bind _output_get (Variables|Default|SetPauseMenuWIdget _returnvalue))
      (UserInterface|Viewport|AddtoViewport _output_get 0)
      (Game|SetGamePaused true)
      (else
        (Variables|Default|SetIsPauseMenuOpened false)
        (Widget|RemovefromParent (Variables|Default|GetPauseMenuWIdget))
        (Game|SetGamePaused false)))))

(event EventBeginPlay
  (CallFunction|InitializeHUD)
  (CallFunction|InitializeLevelUp)
  (bind _asnew_hud (Utilities|Casting|CastToNewHUD (HUD|GetHUD (Game|GetPlayerController 0))))
  (Default|UpdateText (Variables|/Game/Blueprints/NewHUD.NewHUD_C|GetUI_Ref _asnew_hud))
  (Variables|Default|SetDashStamina 1.0)
  (Variables|Default|SetBombCount 0.0))

(event EventPlayerDie
  (if (not (Variables|Default|GetGodMode))
    (Utilities|FlowControl|DoOnce false
      (:Completed
        (bind _asprog_gameplay_proto_game_state (Utilities|Casting|CastToProgGameplayProtoGameState (Game|GetGameState)))
        (Class|ProgGameplayProtoGameState|EndGame _asprog_gameplay_proto_game_state false)))))

(event EventTick
  (params (DeltaSeconds :type Float%20%28single-precision%29)))

(event Input|KeyboardEvents|W
  (params (Key :type Key%20Structure :default "None"))
  (:Pressed
    (bind _isa (Utilities|FlowControl|FlipFlop)
      (:A
        _)
      (:B
        _))
    (bind _output_get (Variables|Default|SetGodMode _isa))
    (Development|PrintString (Utilities|String|Append "God mod : " (Utilities|String|ToString(Boolean) _output_get)) true false "(R=0.000000,G=0.660000,B=1.000000,A=1.000000)" 5.0)))

(event Input|KeyboardEvents|SpaceBar
  (params (Key :type Key%20Structure :default "None"))
  ;[1 0.9997 0] Dash
  (:Pressed
    (if (Variables|Default|GetCanDash)
      (Variables|Default|SetDashStamina 0.0)
      (Variables|Default|SetCanDash false)
      (Variables|Default|SetOldVelocity (Variables|/Script/Engine.MovementComponent|GetVelocity (Variables|Character|GetCharacterMovement)))
      (Variables|/Script/Engine.MovementComponent|SetVelocity (Variables|Character|GetCharacterMovement) (* (Transformation|GetActorForwardVector) 2e+03))
      (Components|Activation|SetActive (Variables|Default|GetDashEffect) true true)
      (CameraShakes|StartCameraShake (Game|GetPlayerCameraManager 0) "/Game/VFX/DashCameraShake_CS.DashCameraShake_CS_C" 1.0 "CameraLocal" "0, 0, 0")
      (Audio|PlaySoundatLocation "/Game/Sounds/Recoil_Blast_2.Recoil_Blast_2" "0, 0, 0" "0, 0, 0" 1.0 1.0 0.0 0 0 0 0)
      (Variables|/Script/ProgGameplayProto.Health|SetIsInvincible (Variables|Default|GetHealth) true)
      (Utilities|FlowControl|Delay 0.2)
      (Variables|/Script/ProgGameplayProto.Health|SetIsInvincible (Variables|Default|GetHealth) false)
      (Components|Activation|SetActive (Variables|Default|GetDashEffect) false false)
      (Variables|/Script/Engine.MovementComponent|SetVelocity (Variables|Character|GetCharacterMovement) (Variables|Default|GetOldVelocity))
      (Utilities|FlowControl|Delay (Variables|Default|GetDashCD))
      (Variables|Default|SetDashStamina 1.0)
      (Variables|Default|SetCanDash true))))

(event Input|KeyboardEvents|B
  (params (Key :type Key%20Structure :default "None"))
  ;[0 0 0] Spawn Bomba
  (:Pressed
    (if (Variables|Default|GetCanBomb)
      (Variables|Default|SetBombCount 1.0)
      (Variables|Default|SetCanBomb false)
      (bind _returnvalue (Game|SpawnActorfromClass "/Game/Blueprints/Items/Bomba_BP.Bomba_BP_C" (Transformation|GetWorldTransform (Variables|Character|GetMesh)) "Undefined" "MultiplyWithRoot" 0 (Variables|Default|GetDamage_Amount) 0))
      (Default|Explode _returnvalue)
      (Utilities|FlowControl|Delay 2e+01)
      (Variables|Default|SetCanBomb true)
      (Variables|Default|SetBombCount 0.0))))

(event Input|KeyboardEvents|Add
  (params (Key :type Key%20Structure :default "None"))
  (:Pressed
    (Utilities|Time|SetGlobalTimeDilation (+ (Class|GameplayStatics|GetGlobalTimeDilation) 2.0))))

(event Input|KeyboardEvents|Subtract
  (params (Key :type Key%20Structure :default "None"))
  (:Pressed
    (Utilities|Time|SetGlobalTimeDilation (- (Class|GameplayStatics|GetGlobalTimeDilation) 2.0))))

(fn ConstructionScript)

(fn InitializeHUD
  (bind _returnvalue (UserInterface|CreateWidget "/Game/UI/GameHUD_UW.GameHUD_UW_C"))
  (UserInterface|Viewport|AddtoViewport _returnvalue 0)
  (Default|Initialize _returnvalue (Variables|Default|GetHealth) (Variables|Default|GetExperience)))

(fn InitializeLevelUp
  (bind _returnvalue (UserInterface|CreateWidget "/Game/UI/LevelUp_UW.LevelUp_UW_C"))
  (Variables|Default|SetLevelUpUI _returnvalue)
  (EventDispatchers|BindEventtoOnLevelUp (Variables|Default|GetExperience) (EventDispatchers|CreateEvent :!event Custom|OnLevelUp)))