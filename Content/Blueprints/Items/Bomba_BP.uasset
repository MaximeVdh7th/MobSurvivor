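; Bomb item that, when Explode is called, burns a fuse for a few seconds before blowing up and damaging nearby enemies.
; The fuse stage plays particles and sound, then the blast adds explosion effects, a camera shake and a radial force impulse.
; A sphere overlap sized to the RadialForce radius finds BaseEnemy_BP pawns and reduces their Health component.
; The actor then destroys itself.
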(event Custom|Explode
  (bind _p_litfuse (Variables|Default|GetP_LitFuse))
  (Components|Activation|Activate _p_litfuse false)
  (Audio|PlaySoundatLocation "/Game/Sounds/FRWKComr_InsJ_Fireworks_Launch_Close_01-03.FRWKComr_InsJ_Fireworks_Launch_Close_01-03" (Transformation|GetActorLocation) "0, 0, 0" 1.0 1.0 0.0 0 0 0 0)
  (Utilities|FlowControl|Delay 3.0)
  (Components|Activation|Deactivate _p_litfuse)
  (Components|Activation|Activate (Variables|Default|GetExplosion) false)
  (Audio|PlaySoundatLocation "/Game/Sounds/explosion_large_no_tail_03.explosion_large_no_tail_03" (Transformation|GetActorLocation) "0, 0, 0" 1.0 1.0 0.0 0 0 0 0)
  (CameraShakes|StartCameraShake (Game|GetPlayerCameraManager 0) "/Game/VFX/BombCameraShake_CS.BombCameraShake_CS_C" 1.0 "CameraLocal" "0, 0, 0")
  (Class|RadialForceComponent|FireImpulse (Variables|Default|GetRadialForce))
  (bind _outactors (Collision|SphereOverlapActors (Transformation|GetActorLocation) (Variables|/Script/Engine.RadialForceComponent|GetRadius (Variables|Default|GetRadialForce)) (Utilities|Array|MakeArray "ObjectTypeQuery3") "/Game/Blueprints/Targets/BaseEnemy_BP.BaseEnemy_BP_C"))
  (for _array_element _outactors
    (Class|Health|AddHealth (Actor|GetComponentbyClass _array_element "/Script/ProgGameplayProto.Health") -5e+01))
  (Actor|DestroyActor))

(fn ConstructionScript)