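; Base enemy Blueprint with 30 health that takes damage from overlapping weapon projectiles and supports melee, ranged and healer behaviors.
; Melee waits, then checks range, facing cone and line of sight before dealing damage and spawning Niagara VFX.
; Ranged attacks spawn projectiles aimed at the player, gated by fire rate and magazine reload.
; Healer support sphere-searches for a damaged ally to store as ProtectedBean and provides healing VFX events.
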(event Custom|MeleeVFX
  ;[0.5231 0.07498 0.485 0.5] Melee VFX
  (Niagara|SpawnSystematLocation "/Game/Materials/VFX/MeleePanner_NS.MeleePanner_NS" (Transformation|GetActorLocation) (Transformation|GetActorRotation)))

(event EventTick
  (params (DeltaSeconds :type Float%20%28single-precision%29))
  ;[1 1 1] Garbage to test rotation
)

(event Collision|EventActorBeginOverlap
  (params (OtherActor :type Actor%20Object%20Reference))
  (bind _asweapon_projectile_bp (Utilities|Casting|CastToWeaponProjectile_BP OtherActor))
  (Class|Enemy|TakeDamage _asweapon_projectile_bp))

(event EventProjectileBP
  (params (Dir :type Vector :default "0, 0, 0"))
  ;[0.07035 0.1257 0.276] Distance Attack Projectile
  (Variables|Default|SetCanDoDistanceAttack false)
  (Utilities|FlowControl|Delay 0.2)
  (bind _returnvalue (Game|SpawnActorfromClass "/Game/Blueprints/Targets/EnemyProjectile_BP.EnemyProjectile_BP_C" (Math|Transform|MakeTransform (Transformation|GetActorLocation) (Math|Conversions|RotationFromXVector Dir) "1.000000,1.000000,1.000000") "AlwaysSpawn" "MultiplyWithRoot" 0 0))
  (Class|EnemyProjectile|Initialize _returnvalue (Utilities|ToPlayer) 2e+01 1e+01 5e+02 1.0)
  (Utilities|FlowControl|Sequence
    (:then_0
      ;;[1 1 1 1 14] Try to melee after shot, follow the player too
      (Utilities|FlowControl|Delay 0.2)
      (Class|Enemy|ReleaseDistance))
    (:then_1
      (bind _result (Math|Integer|IncrementInt (Variables|EnemyParameters|GetMagConsommation))
        (:%20%20
          (if (>= _result (Variables|Default|GetMagSize))
            (Variables|EnemyParameters|SetMagConsommation 0))
          ;;[1 1 1] Reload time (to not spam distance attack)
          (Utilities|FlowControl|Delay (Math|Float|SelectFloat (Variables|Default|GetReloadTime) (Variables|Default|GetFireRate) (>= _result (Variables|Default|GetMagSize))))
          (Variables|Default|SetCanDoDistanceAttack true))))))

(event EventAttackBP
  (params (Target :type Actor%20Object%20Reference))
  (bind _returnvalue (Transformation|GetActorLocation))
  (bind _returnvalue_2 (Transformation|GetActorLocation Target))
  (bind _returnvalue_3 (Transformation|GetActorRotation))
  (bind _returnvalue_4 (Transformation|GetActorRotation))
  (bind _meleeangle (Variables|Default|GetMeleeAngle))
  (bind _meleerange (Variables|Default|GetMeleeRange))
  (bind _returnvalue_5 (Math|Rotator|GetRotationXVector _returnvalue_4))
  (bind _returnvalue_6 (- _returnvalue_2 _returnvalue))
  (bind _returnvalue_7 (* _meleeangle 0.5))
  (bind _returnvalue_8 (Math|Vector|Normalize (Math|Vector|MakeVector (.x _returnvalue_6) (.y _returnvalue_6) 0.0)))
  (bind _returnvalue_9 (Math|Vector|DotProduct _returnvalue_8 (Math|Vector|MakeVector (.x _returnvalue_5) (.y _returnvalue_5) 0.0)))
  (bind _returnvalue_10 (- 1.0 _returnvalue_9))
  (bind _returnvalue_11 (* _returnvalue_10 1.8e+02))
  ;[0.1927 0.06266 0.06266] Melee Attack
  (Utilities|FlowControl|Delay (Variables|Default|GetTimeToAttack))
  ;;[1 1 1] Test distance
  (if (> (* _meleerange _meleerange) (+ (* (.x _returnvalue_6) (.x _returnvalue_6)) (* (.x _returnvalue_6) (.x _returnvalue_6))))
    (if (and (< _returnvalue_11 (+ (.yaw _returnvalue_3) _returnvalue_7)) (> _returnvalue_11 (- (.yaw _returnvalue_3) _returnvalue_7)))
      (bind _returnvalue_12 (Collision|LineTraceForObjects (Transformation|GetActorLocation) (Transformation|GetActorLocation Target) (Utilities|Array|MakeArray "ObjectTypeQuery1" "ObjectTypeQuery1") false 0 "None"))
      (if _returnvalue_12
        (Variables|Default|SetMeleeAttack false)
        (else
          (Class|Enemy|DoDamage Target)
          (CallFunction|MeleeVFX)))
      (else
        (Variables|Default|SetMeleeAttack false :!label _label)))
    (else
      (goto _label))))

(event EventBeginPlay
  (bind _health (Variables|Default|GetHealth))
  ;[0.8118 0.1866 0.1866 0.116] Set Life
  (Variables|/Script/ProgGameplayProto.Health|SetMaxHealth _health 3e+01)
  (Variables|/Script/ProgGameplayProto.Health|SetCurrentHealth _health 3e+01))

(event EventHealVFX
  (params (ProtectionPos :type Vector :default "0, 0, 0"))
  (bind _returnvalue (Niagara|SpawnSystematLocation "/Game/Materials/VFX/Heal_NS.Heal_NS" (Transformation|GetActorLocation) (Transformation|GetActorRotation)))
  (Class|NiagaraComponent|SetVariablePosition _returnvalue "TargetPos" ProtectionPos))

(event EventTrytoFindAllies
  ;[0.1868 0.04405 0.06722 0.5] Find someone to Heal
  (bind _outactors (Collision|SphereOverlapActors (Transformation|GetActorLocation) 3e+02 (Utilities|Array|MakeArray "ObjectTypeQuery3") "BaseEnemy_BP_C" (Utilities|Array|MakeArray self)))
  (bind _array_element (Utilities|Array|ForEachLoopwithBreak _outactors :!label _label)
    (:LoopBody
      (bind _asbase_enemy_bp (Utilities|Casting|CastToBaseEnemy_BP _array_element))
      (if (< (Variables|/Script/ProgGameplayProto.Health|GetCurrentHealth (Actor|GetComponentbyClass _asbase_enemy_bp "/Script/ProgGameplayProto.Health")) (Variables|/Script/ProgGameplayProto.Health|GetMaxHealth (Actor|GetComponentbyClass _asbase_enemy_bp "/Script/ProgGameplayProto.Health")))
        (Utilities|FlowControl|Sequence
          (:then_0
            (Variables|Default|SetProtectedBean _asbase_enemy_bp))
          (:then_1
            (goto _label Break)))
        (else
          (Variables|Default|SetProtectedBean 0))))))

(event EventStartHealing
  (Niagara|SpawnSystemAttached "/Game/Materials/VFX/WillHeal_NS.WillHeal_NS" (Variables|Default|GetMesh) "None" "0, 0, 0" "0, 0, 0" "SnapToTarget" true))

(fn ConstructionScript)